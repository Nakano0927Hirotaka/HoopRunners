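; BP_EnemyCharacter is an enemy character that sends players to a cage when its capsule hits them.
; On a hit with a BP_FirstPersonCharacter, only the server teleports that player above the first actor tagged "Cage" and sets its Cageing flag.
; It then asks BP_GameMode to check whether all players are caged.
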(event `self.CapsuleComponent.OnComponentHit`
  (params (HitComponent :type "PrimitiveComponent Object Reference") (OtherActor :type "Actor Object Reference") (OtherComp :type "PrimitiveComponent Object Reference") (NormalImpulse :type "Vector Structure") (Hit :type "HitResult Structure (by ref)"))
  (bind _asbp_first_person_character (cast `/Game/FirstPerson/Blueprints/BP_FirstPersonCharacter` OtherActor))
  (`/Engine/EditorBlueprintResources/ActorMacros.Switch Has Authority`
    (:`Authority`
      (bind _outactors (`GameplayStatics.GetAllActorsWithTag` "Cage"))
      (`self.K2_SetActorLocation` _asbp_first_person_character (+ (`self.K2_GetActorLocation` (`|GetArrayItem` _outactors)) (0.0 0.0 200.0)) false true)
      (set `/Game/FirstPerson/Blueprints/BP_FirstPersonCharacter.Cageing` true _asbp_first_person_character)
      (bind _asbp_game_mode (cast `/Game/Saver/BP_GameMode` (`GameplayStatics.GetGameMode`)))
      (`/Game/Saver/BP_GameMode.CheckAllPlayersCaged` _asbp_game_mode))))

(fn `UserConstructionScript`)