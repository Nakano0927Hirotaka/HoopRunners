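; Game mode Blueprint that ends the game when every player character is caged.
; CheckAllPlayersCaged scans all first-person characters' Cageing flags and, if all are set, calls ClientShowGameOver on each player controller.
; Separate Multicast-named game-over and game-clear events add their widget, switch to UI-only input and pause.
; BeginPlay restores unpaused game-only input, and controller swaps print class names for debugging.
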(event `self.ReceiveBeginPlay`
  (set `self.AllCaged` true)
  (`GameplayStatics.SetGamePaused` false)
  (`WidgetBlueprintLibrary.SetInputMode_GameOnly` (`GameplayStatics.GetPlayerController` 0)))

(event `self.K2_OnSwapPlayerControllers`
  (params (OldPC :type "PlayerController Object Reference") (NewPC :type "PlayerController Object Reference"))
  (`KismetSystemLibrary.PrintString` (`KismetSystemLibrary.GetClassDisplayName` (`GameplayStatics.GetObjectClass` OldPC)))
  (`KismetSystemLibrary.PrintString` (`KismetSystemLibrary.GetClassDisplayName` (`GameplayStatics.GetObjectClass` NewPC))))

(event `CheckAllPlayersCaged`
  (set `self.AllCaged` true)
  (bind _outactors (`GameplayStatics.GetAllActorsOfClass` "/Game/FirstPerson/Blueprints/BP_FirstPersonCharacter.BP_FirstPersonCharacter_C"))
  (for _array_element _outactors
    (if (not (`/Game/FirstPerson/Blueprints/BP_FirstPersonCharacter.Cageing` _array_element))
      (set `self.AllCaged` false)))
  (if (`self.AllCaged`)
    (bind _outactors_2 (`GameplayStatics.GetAllActorsOfClass` "/Game/FirstPerson/Blueprints/BP_FirstPersonPlayerController.BP_FirstPersonPlayerController_C"))
    (for _array_element_2 _outactors_2
      (`/Game/FirstPerson/Blueprints/BP_FirstPersonPlayerController.Client_ShowGameOver` _array_element_2))))

(event `Multicast_ShowGameOver`
  (`|ExecutionSequence`
    (:`then_0`
      (bind _returnvalue (`|CreateWidget` "/Game/Saver/GameOverUI.GameOverUI_C"))
      (`UserWidget.AddToViewport` _returnvalue 0))
    (:`then_1`
      (`WidgetBlueprintLibrary.SetInputMode_UIOnlyEx` (`GameplayStatics.GetPlayerController` 0) null "LockOnCapture"))
    (:`then_2`
      (`GameplayStatics.SetGamePaused` true))))

(event `Multicast_ShowGameClear`
  (`|ExecutionSequence`
    (:`then_0`
      (bind _returnvalue (`|CreateWidget` "/Game/Saver/GameCearUI.GameCearUI_C"))
      (`UserWidget.AddToViewport` _returnvalue 0))
    (:`then_1`
      (`WidgetBlueprintLibrary.SetInputMode_UIOnlyEx` (`GameplayStatics.GetPlayerController` 0) null "LockOnCapture"))
    (:`then_2`
      (`GameplayStatics.SetGamePaused` true))))

(fn `UserConstructionScript`)